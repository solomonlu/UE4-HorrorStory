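; BP_Door_Metal_01 is a double sliding door that opens when a Character enters its trigger and closes when one leaves.
; BeginPlay caches the relative locations of both door panels as their closed positions.
; Trigger overlaps call OpenDoor and CloseDoor, which play the DoorSlideTimer timeline from the start or reverse it from the end.
; The timeline's OpenRatio slides the panels apart along local Y from those cached positions.
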(event `self.ReceiveBeginPlay`
  (set `self.Door1Offset` (`SceneComponent.RelativeLocation` (`self.Door1`)))
  (set `self.Door2Offset` (`SceneComponent.RelativeLocation` (`self.Door2`)))
  (bind (_direction _openratio) (`Timeline|DoorSlideTimer` :!via `Stop`)
    (:`Update`
      (bind _returnvalue (`KismetMathLibrary.MakeVector` 0.0 (* _openratio 200.0)))
      (`SceneComponent.K2_SetRelativeLocation` (- (`self.Door1Offset`) _returnvalue))
      (`SceneComponent.K2_SetRelativeLocation` (+ (`self.Door2Offset`) _returnvalue)))))

(event `OpenDoor`
  (`TimelineComponent.PlayFromStart`))

(event `CloseDoor`
  (`TimelineComponent.ReverseFromEnd`))

(event `self.DoorTrigger.OnComponentBeginOverlap`
  (params (OverlappedComponent :type "PrimitiveComponent Object Reference") (OtherActor :type "Actor Object Reference") (OtherComp :type "PrimitiveComponent Object Reference") (OtherBodyIndex :type Integer) (bFromSweep :type Boolean) (SweepResult :type "HitResult Structure (by ref)"))
  (cast `Character` OtherActor)
  (`self.OpenDoor`))

(event `self.DoorTrigger.OnComponentEndOverlap`
  (params (OverlappedComponent :type "PrimitiveComponent Object Reference") (OtherActor :type "Actor Object Reference") (OtherComp :type "PrimitiveComponent Object Reference") (OtherBodyIndex :type Integer))
  (cast `Character` OtherActor)
  (`self.CloseDoor`))

(fn `UserConstructionScript`)