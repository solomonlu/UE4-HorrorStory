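; BP_GameMode assigns horror master and hero roles as players join and triggers game over when the heroes are down.
; On PostLogin, the first player possesses a BP_CommanderCharacter spawned at a PlayerStart as horror master, unless NoHorrorMasterMode is set.
; Other players get a sequential HeroIndex on their BP_PlayerController.
; OneHeroDown counts downed heroes and, at four, replaces all widgets with UI_GameOver for player controller 0.
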(event `self.K2_PostLogin`
  (params (NewPlayer :type "PlayerController Object Reference"))
  (bind _asbp_player_controller (cast `/Game/HorrorStory/ZombieWorldScene/Blueprints/Character/Hero/BP_PlayerController` NewPlayer))
  (bind _returnvalue (`self.GetNumPlayers`))
  (bind _returnvalue_2 (- _returnvalue (select `bool` (`self.NoHorrorMasterMode`) :`false` 1)))
  (if (== _returnvalue_2 0)
    ;[1 1 1] horror master
    (set `/Game/HorrorStory/ZombieWorldScene/Blueprints/Character/Hero/BP_PlayerController.IsHorrorMaster` true _asbp_player_controller)
    (bind _outactors (`GameplayStatics.GetAllActorsOfClass` "/Script/Engine.PlayerStart"))
    (bind _returnvalue_3 (`|SpawnActorFromClass` "/Game/HorrorStory/ZombieWorldScene/Blueprints/Character/Commander/BP_CommanderCharacter.BP_CommanderCharacter_C" (`self.GetTransform` (`KismetArrayLibrary.Array_Get` _outactors)) "Undefined" "OverrideRootScale"))
    (`Controller.Possess` _asbp_player_controller _returnvalue_3)
    (else
      ;[1 1 1] hero
      (set `/Game/HorrorStory/ZombieWorldScene/Blueprints/Character/Hero/BP_PlayerController.IsHorrorMaster` false _asbp_player_controller)
      (set `/Game/HorrorStory/ZombieWorldScene/Blueprints/Character/Hero/BP_PlayerController.HeroIndex` (- _returnvalue_2 1) _asbp_player_controller))))

(event `OneHeroDown`
  (bind _result (`/Engine/EditorBlueprintResources/StandardMacros.IncrementInt` (`self.DownHero`))
    (:`  `
      (if (>= _result 4)
        (`WidgetLayoutLibrary.RemoveAllWidgets`)
        (bind _returnvalue (`|CreateWidget` "/Game/HorrorStory/ZombieWorldScene/Blueprints/UI/UI_GameOver.UI_GameOver_C" (`GameplayStatics.GetPlayerController` 0)))
        (`UserWidget.AddToViewport` _returnvalue 0)))))

(fn `UserConstructionScript`)