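; Game mode for the Zombie World scene that decides whether the master or the heroes win the match.
; It collects each joining player controller on PostLogin, then calls NotifySettlement on all of them with a flag for a master win.
; Tick fires a one-time master win when the game state's timer runs out, while MasterBodyDown gives heroes the win.
; The hero-down kill count path is marked unused, and EnergyCudeDown is an empty stub.
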(event `self.K2_PostLogin`
  (params (NewPlayer :type "PlayerController Object Reference"))
  (`parent.K2_PostLogin` NewPlayer)
  (bind _asbp_zombie_world_player_controller (cast `/Game/HorrorStory/ZombieWorldScene/Blueprints/GameModeEtc/BP_ZombieWorldPlayerController` NewPlayer))
  (`KismetArrayLibrary.Array_AddUnique` (`self.PlayerControllers`) _asbp_zombie_world_player_controller))

(event `self.ReceiveTick`
  (params (DeltaSeconds :type "Float (single-precision)"))
  ;[1 1 1] Win or lose
  ;;[1 1 1] time exhaused or all hero down, master win
  (if (<= (`/Game/HorrorStory/ZombieWorldScene/Blueprints/GameModeEtc/BP_ZombieWorldGameState.GetGameRemainTime` (cast `/Game/HorrorStory/ZombieWorldScene/Blueprints/GameModeEtc/BP_ZombieWorldGameState` (`GameplayStatics.GetGameState`) :!pure true)) 0.0)
    (`/Engine/EditorBlueprintResources/StandardMacros.DoOnce` false
      (:`Completed`
        (for _array_element (`self.PlayerControllers`)
          (`/Game/HorrorStory/ZombieWorldScene/Blueprints/GameModeEtc/BP_ZombieWorldPlayerController.NotifySettlement` _array_element true))))))

(event `OneHeroDown`
  ;[1 1 1] Win or lose
  ;;[1 1 1] time exhaused or all hero down, master win
  ;;;[1 0.025 0.025] no use this
  (`/Engine/EditorBlueprintResources/StandardMacros.IncrementInt` (`self.KillHeroCount`)
    (:`  `
      (bind _returnvalue (`self.GetNumPlayers`))
      (if (== (- _returnvalue (`self.KillHeroCount`)) 1)
        (for _array_element (`self.PlayerControllers`)
          (`/Game/HorrorStory/ZombieWorldScene/Blueprints/GameModeEtc/BP_ZombieWorldPlayerController.NotifySettlement` _array_element true))))))

(event `MasterBodyDown`
  ;[1 1 1] Win or lose
  ;;[1 1 1] master body destroyed, heroes win
  (for _array_element (`self.PlayerControllers`)
    (`/Game/HorrorStory/ZombieWorldScene/Blueprints/GameModeEtc/BP_ZombieWorldPlayerController.NotifySettlement` _array_element false)))

(event `EnergyCudeDown`
  ;[1 1 1] Win or lose
)

(fn `UserConstructionScript`)