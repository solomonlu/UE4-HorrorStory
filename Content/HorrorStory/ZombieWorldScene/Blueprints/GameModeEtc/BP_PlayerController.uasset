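; Player controller for an asymmetric zombie mode that serves either a Horror Master or a Hero, branching on IsHorrorMaster.
; It creates role-specific HUD and game-over widgets, plus an in-game menu toggled by I or Escape.
; The Master drags to pan its pawn through a tick-fed gate and spawns zombies on the navmesh under the cursor, limited by a cooldown.
; The Hero's control rotation follows the cursor hit point.
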(event `InitUI`
  (`KismetSystemLibrary.Delay` 0.5)
  (if (`self.IsHorrorMaster`)
    ;[1 1 1] Master UI
    (bind _returnvalue (`|CreateWidget` "/Game/HorrorStory/ZombieWorldScene/Blueprints/UI/UI_MasterInGame.UI_MasterInGame_C" self))
    (`UserWidget.AddToViewport` _returnvalue 0)
    (else
      ;[1 1 1] Hero UI
      (bind _returnvalue_2 (`|CreateWidget` "/Game/HorrorStory/ZombieWorldScene/Blueprints/UI/UI_HeroInGame.UI_HeroInGame_C" self))
      (`UserWidget.AddToViewport` _returnvalue_2 0)))
  ;[1 1 1] Also creating our IngameMenu. All of our GameModes have this
  (bind _returnvalue_3 (`|CreateWidget` "/Game/HorrorStory/Common/Blueprints/UI/IngameMenu/W_InGameMenu.W_InGameMenu_C" self "/Game/HorrorStory/Common/Blueprints/UI/IngameMenu/W_PlayerListEntryWidget.W_PlayerListEntryWidget_C"))
  (set `self.InGameMenuWidgetRef` _returnvalue_3))

(event `NotifyMasterIsWin`
  (params (IsWin :type Boolean) (KillCount :type Integer))
  (if (`self.IsHorrorMaster`)
    (`WidgetLayoutLibrary.RemoveAllWidgets`)
    (bind _returnvalue (`|CreateWidget` "/Game/HorrorStory/ZombieWorldScene/Blueprints/UI/UI_MasterGameOver.UI_MasterGameOver_C" self IsWin KillCount))
    (`UserWidget.AddToViewport` _returnvalue 0)
    (`WidgetBlueprintLibrary.SetInputMode_UIOnlyEx` self)))

(event `NotifyHeroIsWin`
  (params (IsWin :type Boolean))
  (if (not (`self.IsHorrorMaster`))
    (`WidgetLayoutLibrary.RemoveAllWidgets`)
    (bind _returnvalue (`|CreateWidget` "/Game/HorrorStory/ZombieWorldScene/Blueprints/UI/UI_HeroGameOver.UI_HeroGameOver_C" self IsWin))
    (`UserWidget.AddToViewport` _returnvalue 0)
    (`WidgetBlueprintLibrary.SetInputMode_UIOnlyEx` self)))

(event `self.ReceiveBeginPlay`
  ;[1 1 1] Give focus to the Game
  (`WidgetBlueprintLibrary.SetFocusToGameViewport`)
  (`WidgetBlueprintLibrary.SetInputMode_GameOnly` (`GameplayStatics.GetPlayerController` 0)))

(event `Key|I`
  (params (Key :type "Key Structure" :default "AnyKey"))
  ;[0 0 0] Open our ingame menu
  (:`Pressed`
    (if (`self.bIngameMenuOpen`) :!label _label
      (`Widget.RemoveFromParent` (`self.InGameMenuWidgetRef`))
      (`WidgetBlueprintLibrary.SetInputMode_GameOnly` self)
      (set `self.bIngameMenuOpen` false)
      (set `self.bShowMouseCursor` false)
      (else
        (`UserWidget.AddToViewport` (`self.InGameMenuWidgetRef`) 0)
        (`WidgetBlueprintLibrary.SetInputMode_UIOnlyEx` self (`self.InGameMenuWidgetRef`))
        (set `self.bIngameMenuOpen` true)
        (set `self.bShowMouseCursor` true)))))

(event `Key|Escape`
  (params (Key :type "Key Structure" :default "AnyKey"))
  ;[0 0 0] Open our ingame menu
  (:`Pressed`
    (goto _label)))

(event `SpawnZombie`
  (params (SpawnLocation :type "Vector Structure"))
  ;[1 0 0.00868] spawn zombie,TODO:Move to character?
  (`|SpawnActorFromClass` "/Game/HorrorStory/ZombieWorldScene/Blueprints/Character/Zombie/BP_Zombie.BP_Zombie_C" (`KismetMathLibrary.MakeTransform` SpawnLocation) "AdjustIfPossibleButAlwaysSpawn" "OverrideRootScale"))

(event `InputAction|RightTouch`
  (params (Key :type "Key Structure" :default "AnyKey"))
  ;[1 0 0.00868] spawn zombie,TODO:Move to character?
  (:`Pressed`
    (if (`self.IsHorrorMaster`)
      (if (<= (`self.CurrentSpawnCoolDown`) 0.0)
        (`self.SpawnZombie` (+ (`NavigationSystem.ProjectPointToNavigation` (`.Location` (`GameplayStatics.BreakHitResult` (`self.GetHitResultUnderCursorByChannel` "TraceTypeQuery1")))) (0.0 0.0 50.0)))
        (set `self.CurrentSpawnCoolDown` (`self.SpawnCooldown`))))))

(event `InputAction|LeftTouch` :consume false
  (params (Key :type "Key Structure" :default "AnyKey"))
  (bind (_locationx _locationy) (`self.GetMousePosition`))
  (bind (_locationx_2 _locationy_2) (`self.GetMousePosition`))
  (bind (_returnvalue_x _returnvalue_y) (`KismetMathLibrary.BreakVector` (- (`self.TouchStartMousePosition`) (`KismetMathLibrary.MakeVector` _locationx_2 _locationy_2))))
  ;[1 1 1] Record mouse and commander position when touch start
  (:`Pressed`
    (set `self.TouchStartMousePosition` (`KismetMathLibrary.MakeVector` _locationx _locationy))
    (set `self.TouchStartCommanderPosition` (`self.K2_GetActorLocation` (`self.K2_GetPawn`)))
    (goto _label_2 :!via `Open`))
  (:`Released`
    (goto _label_2 :!via `Close`)))

(event `self.ReceiveTick`
  (params (DeltaSeconds :type "Float (single-precision)"))
  (bind (_locationx _locationy) (`self.GetMousePosition`))
  (bind (_returnvalue_x _returnvalue_y) (`KismetMathLibrary.BreakVector` (- (`self.TouchStartMousePosition`) (`KismetMathLibrary.MakeVector` _locationx _locationy))))
  ;[1 0.01 0.01] TODO
  (`|ExecutionSequence`
    (:`then_0`
      (`/Engine/EditorBlueprintResources/StandardMacros.IsValid` (`self.K2_GetPawn`)
        (:`Is Valid`
          (if (`self.IsHorrorMaster`)
            (`/Engine/EditorBlueprintResources/StandardMacros.Gate` true :!label _label_2 ; While key is pressed...
              (:`Exit`
                (`self.K2_SetActorLocation` (`self.K2_GetPawn`) (+ (`self.TouchStartCommanderPosition`) (* (* (`KismetMathLibrary.MakeVector` _returnvalue_y (* _returnvalue_x -1.0 (`KismetMathLibrary.DegCos` 60.0))) -1.0) (`self.MouseMoveScale`))) false false)))
            (else
              ;[1 1 1] hero use mouse to rotate
              (`self.SetControlRotation` (`KismetMathLibrary.FindLookAtRotation` (`self.K2_GetActorLocation` (`self.K2_GetPawn`)) (`.Location` (`GameplayStatics.BreakHitResult` (`self.GetHitResultUnderCursorByChannel` "TraceTypeQuery1"))))))))))
    (:`then_1`
      (if (> (`self.CurrentSpawnCoolDown`) 0.0)
        (set `self.CurrentSpawnCoolDown` (- (`self.CurrentSpawnCoolDown`) DeltaSeconds))))))

(fn `UserConstructionScript`)