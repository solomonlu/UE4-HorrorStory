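; BP_EnergyCube is a destructible energy cube actor that reports its destruction to the zombie world game mode.
; The construction script fills Health from MaxHealth, and AnyDamage subtracts from it until it reaches zero, firing OnDeath through a DoOnce.
; OnDeath notifies BP_ZombieWorldGameMode via EnergyCudeDown on authority before destroying the actor, while the remote branch goes straight to destruction.
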(event `self.ReceiveAnyDamage`
  (params (Damage :type "Float (single-precision)") (DamageType :type "DamageType Object Reference") (InstigatedBy :type "Controller Object Reference") (DamageCauser :type "Actor Object Reference"))
  (bind _output_get (set `self.Health` (- (`self.Health`) Damage)))
  (if (<= _output_get 0.0)
    (`/Engine/EditorBlueprintResources/StandardMacros.DoOnce` false
      (:`Completed`
        (`self.OnDeath`)))))

(event `OnDeath`
  (`/Engine/EditorBlueprintResources/ActorMacros.Switch Has Authority`
    (:`Authority`
      (bind _asbp_zombie_world_game_mode (cast `/Game/HorrorStory/ZombieWorldScene/Blueprints/GameModeEtc/BP_ZombieWorldGameMode` (`GameplayStatics.GetGameMode`)))
      (`/Game/HorrorStory/ZombieWorldScene/Blueprints/GameModeEtc/BP_ZombieWorldGameMode.EnergyCudeDown` _asbp_zombie_world_game_mode))
    (:`Remote`
      _))
  (`self.K2_DestroyActor`))

(fn `UserConstructionScript`
  (set `self.Health` (`self.MaxHealth`)))