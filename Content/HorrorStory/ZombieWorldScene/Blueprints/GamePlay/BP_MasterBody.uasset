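; BP_MasterBody is a destructible actor in the zombie world mode that stays immune to damage while any BP_EnergyCube exists in the level.
; Damage taken during immunity calls a tip event that shows its TextRender for five seconds.
; Once no cubes remain, damage reduces Health, initialized from MaxHealth, until death fires once.
; On death, the authority notifies BP_ZombieWorldGameMode through MasterBodyDown, and the actor is destroyed.
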(event `self.ReceiveAnyDamage`
  (params (Damage :type "Float (single-precision)") (DamageType :type "DamageType Object Reference") (InstigatedBy :type "Controller Object Reference") (DamageCauser :type "Actor Object Reference"))
  ;[1 1 1] if energy cube exists, i'm immortal
  (bind _outactors (`GameplayStatics.GetAllActorsOfClass` "/Game/HorrorStory/ZombieWorldScene/Blueprints/GamePlay/BP_EnergyCube.BP_EnergyCube_C"))
  (if (== (`KismetArrayLibrary.Array_Length` _outactors) 0)
    (bind _output_get (set `self.Health` (- (`self.Health`) Damage)))
    (if (<= _output_get 0.0)
      (`/Engine/EditorBlueprintResources/StandardMacros.DoOnce` false
        (:`Completed`
          (`self.OnDeath`))))
    (else
      (`self.MC_ShowTips`))))

(event `MC_ShowTips`
  (`SceneComponent.SetHiddenInGame` (`self.TextRender`) false false)
  (`KismetSystemLibrary.Delay` 5.0)
  (`SceneComponent.SetHiddenInGame` (`self.TextRender`) true false))

(event `OnDeath`
  (`/Engine/EditorBlueprintResources/ActorMacros.Switch Has Authority`
    (:`Authority`
      (bind _asbp_zombie_world_game_mode (cast `/Game/HorrorStory/ZombieWorldScene/Blueprints/GameModeEtc/BP_ZombieWorldGameMode` (`GameplayStatics.GetGameMode`)))
      (`/Game/HorrorStory/ZombieWorldScene/Blueprints/GameModeEtc/BP_ZombieWorldGameMode.MasterBodyDown` _asbp_zombie_world_game_mode))
    (:`Remote`
      _))
  (`self.K2_DestroyActor`))

(fn `UserConstructionScript`
  (set `self.Health` (`self.MaxHealth`)))