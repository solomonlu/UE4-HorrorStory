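; Playable multiplayer hero for the zombie scene, with world-axis movement, firing and switching between rifle and shotgun.
; Fire and weapon input go through server events to multicasts that drive BPAttackComponent, rotation mode and weapon meshes.
; The anim instance triggers projectile spawning on authority, along controller yaw.
; Damage lowers Health until death ragdolls the mesh and notifies the game mode, while replicated HeroIndex selects body color.
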(event `self.ReceiveBeginPlay`
  (`|ExecutionSequence`
    (:`then_0`
      (`self.OnEquipRangeWeapon` (`self.DefaultWeaponType`)))
    (:`then_1`
      ;[1 1 1] bullet spawn, should not do like this
      (bind _asbpa_hero (cast `/Game/HorrorStory/ZombieWorldScene/Blueprints/Character/Hero/BPA_Hero` (`SkeletalMeshComponent.GetAnimInstance` (`self.Mesh`))))
      (add `/Game/HorrorStory/ZombieWorldScene/Blueprints/Character/Hero/BPA_Hero.SpawnProjectile` _asbpa_hero (delegate `SpawnProjectile`)))
    (:`then_2`
      ;[1 1 1] add myself into ai storage
      (bind _outactors (`GameplayStatics.GetAllActorsOfClass` "/Game/AIBehaviorToolkit/Blueprints/BP_AIStorage.BP_AIStorage_C"))
      (if (> (`KismetArrayLibrary.Array_Length` _outactors) 0)
        (`/Game/AIBehaviorToolkit/Blueprints/BP_AIStorage.AddActorToList` (`KismetArrayLibrary.Array_Get` _outactors) self)))))

(event `SpawnProjectile`
  (bind (_returnvalue_roll _returnvalue_pitch _returnvalue_yaw) (`KismetMathLibrary.BreakRotator` (`self.GetControlRotation`)))
  ;[1 1 1] bullet spawn, should not do like this
  (`/Engine/EditorBlueprintResources/ActorMacros.Switch Has Authority`
    (:`Authority`
      (`/Game/HorrorStory/ZombieWorldScene/Blueprints/Character/Component/AttackComponent/BP_AttackComponent.SpawnBullet` (`self.BP_AttackComponent`) (`KismetMathLibrary.MakeTransform` (`self.K2_GetActorLocation`) (`KismetMathLibrary.MakeRotator` 0.0 0.0 _returnvalue_yaw))))))

(event `self.ReceiveAnyDamage`
  (params (Damage :type "Float (single-precision)") (DamageType :type "DamageType Object Reference") (InstigatedBy :type "Controller Object Reference") (DamageCauser :type "Actor Object Reference"))
  ;[1 1 1] damage and death
  ;;[1 1 1] Reduce Health based on damage
  (bind _output_get (set `self.Health` (- (`self.Health`) Damage)))
  (if (<= _output_get 0.0)
    (`self.OnDeath`)))

(event `self.ReceivePossessed`
  (params (NewController :type "Controller Object Reference"))
  (bind _asbp_player_controller (cast `/Game/HorrorStory/ZombieWorldScene/Blueprints/Character/Hero/BP_PlayerController` NewController))
  (set `self.HeroIndex` (`/Game/HorrorStory/ZombieWorldScene/Blueprints/Character/Hero/BP_PlayerController.HeroIndex` _asbp_player_controller)))

(event `OnDeath`
  (bind _returnvalue (`self.GetController`))
  (bind _capsulecomponent (`self.CapsuleComponent`))
  (bind _mesh (`self.Mesh`))
  ;[1 1 1] damage and death
  (`|ExecutionSequence`
    (:`then_0`
      ;;[1 1 1] Default ragdoll death event
      (`PrimitiveComponent.SetCollisionResponseToAllChannels` _capsulecomponent "ECR_Ignore")
      (`PrimitiveComponent.SetCollisionResponseToChannel` _capsulecomponent "ECC_WorldStatic" "ECR_Block")
      (`PrimitiveComponent.SetCollisionProfileName` _mesh "Ragdoll")
      (`PrimitiveComponent.SetSimulatePhysics` _mesh true)
      (`AnimInstance.Montage_Stop` (`SkeletalMeshComponent.GetAnimInstance` _mesh) 0.0 null)
      ;;[1 1 1] clear tags
      (set `self.Tags` (`|MakeArray` "None" :!type "Name")))
    (:`then_1`
      ;;[1 1 1] notify game mode, one hero down
      (bind _asbp_game_mode (cast `/Game/HorrorStory/ZombieWorldScene/Blueprints/GameModeEtc/BP_GameMode` (`GameplayStatics.GetGameMode`)))
      (`/Game/HorrorStory/ZombieWorldScene/Blueprints/GameModeEtc/BP_GameMode.OneHeroDown` _asbp_game_mode))
    (:`then_2`
      ;;[1 1 1] disable owning client input
      (if (`KismetSystemLibrary.IsValid` _returnvalue)
        (if (`Controller.IsLocalPlayerController` _returnvalue)
          (`WidgetBlueprintLibrary.SetInputMode_UIOnlyEx` (cast `PlayerController` _returnvalue :!pure true)))))))

(event `OnEquipRangeWeapon`
  (params (WeaponType :type "/Game/HorrorStory/ZombieWorldScene/Blueprints/Character/Hero/Weapon/Enum_WeaponType Enum"))
  (`|ExecutionSequence`
    (:`then_0`
      (`/Game/HorrorStory/ZombieWorldScene/Blueprints/Character/Component/AttackComponent/BP_AttackComponent.OnEquipWeapon` (`self.BP_AttackComponent`) WeaponType))
    (:`then_1`
      ;[1 1 1] set which weapon mesh to show
      (`SceneComponent.SetHiddenInGame` (`self.Shotgun`) true false)
      (`SceneComponent.SetHiddenInGame` (`self.AssaultGun`) true false)
      (switch `/Game/HorrorStory/ZombieWorldScene/Blueprints/Character/Hero/Weapon/Enum_WeaponType` WeaponType
        (:`NewEnumerator0`
          (`SceneComponent.SetHiddenInGame` (`self.AssaultGun`) false false))
        (:`NewEnumerator1`
          (`SceneComponent.SetHiddenInGame` (`self.Shotgun`) false false))))))

(event `InputAxis|MoveForward`
  (params (AxisValue :type "Float (single-precision)"))
  ;[1 1 1] Movement
  (`self.AddMovementInput` (1.0 0.0 0.0) AxisValue))

(event `InputAxis|MoveRight`
  (params (AxisValue :type "Float (single-precision)"))
  ;[1 1 1] Movement
  (`self.AddMovementInput` (0.0 1.0 0.0) AxisValue))

(event `InputAction|Fire`
  (params (Key :type "Key Structure" :default "AnyKey"))
  ;[1 1 1] Fire
  (:`Pressed`
    (`self.Server_OnFire` true))
  (:`Released`
    (`self.Server_OnFire` false)))

(event `Server_OnFire`
  (params (IsAttacking :type Boolean))
  ;[1 1 1] Fire
  (`self.MC_OnFire` IsAttacking))

(event `MC_OnFire`
  (params (IsAttacking :type Boolean))
  ;[1 1 1] Fire
  (set `/Game/HorrorStory/ZombieWorldScene/Blueprints/Character/Component/AttackComponent/BP_AttackComponent.IsAttacking` IsAttacking (`self.BP_AttackComponent`))
  (set `CharacterMovementComponent.bOrientRotationToMovement` (not IsAttacking) (`self.CharacterMovement`))
  (set `self.bUseControllerRotationYaw` IsAttacking))

(event `InputAction|EquipLastWeapon`
  (params (Key :type "Key Structure" :default "AnyKey"))
  ;[1 1 1] Equip weapon
  (:`Pressed`
    (`self.Server_OnEquipLastWeapon`)))

(event `InputAction|EquipNextWeapon`
  (params (Key :type "Key Structure" :default "AnyKey"))
  ;[1 1 1] Equip weapon
  (:`Pressed`
    (`self.Server_OnEquipNextWeapon`)))

(event `Server_OnEquipLastWeapon`
  ;[1 1 1] Equip weapon
  (`self.MC_OnEquipWeapon` (cast `/Game/HorrorStory/ZombieWorldScene/Blueprints/Character/Hero/Weapon/Enum_WeaponType` (mod (- (`self.CurrentWeaponType`) 1) (enumliteral `/Game/HorrorStory/ZombieWorldScene/Blueprints/Character/Hero/Weapon/Enum_WeaponType` "NewEnumerator2")))))

(event `Server_OnEquipNextWeapon`
  ;[1 1 1] Equip weapon
  (`self.MC_OnEquipWeapon` (cast `/Game/HorrorStory/ZombieWorldScene/Blueprints/Character/Hero/Weapon/Enum_WeaponType` (mod (+ (`self.CurrentWeaponType`) 1) (enumliteral `/Game/HorrorStory/ZombieWorldScene/Blueprints/Character/Hero/Weapon/Enum_WeaponType` "NewEnumerator2")))))

(event `MC_OnEquipWeapon`
  (params (NewWeapon :type "/Game/HorrorStory/ZombieWorldScene/Blueprints/Character/Hero/Weapon/Enum_WeaponType Enum"))
  ;[1 1 1] Equip weapon
  (bind _output_get (set `self.CurrentWeaponType` NewWeapon))
  ;;[1 1 1] todo:rewrite
  (`self.OnEquipRangeWeapon` _output_get))

(fn `OnRep_Health`)

(fn `OnRep_HeroIndex`
  (`PrimitiveComponent.SetMaterial` (`self.Mesh`) 0 (select `int` (`self.HeroIndex`) :`0` "/Game/AIBehaviorToolkit/Assets/Mannequin/Character/Materials/M_UE4Man_Body_Black_Inst.M_UE4Man_Body_Black_Inst" :`1` "/Game/AIBehaviorToolkit/Assets/Mannequin/Character/Materials/M_UE4Man_Body_Blue_Inst.M_UE4Man_Body_Blue_Inst" :`2` "/Game/AIBehaviorToolkit/Assets/Mannequin/Character/Materials/M_UE4Man_Body_Green_Inst.M_UE4Man_Body_Green_Inst" :`3` "/Game/AIBehaviorToolkit/Assets/Mannequin/Character/Materials/M_UE4Man_Body_Red_Inst.M_UE4Man_Body_Red_Inst" :!type "MaterialInterface Object Reference")))

(fn `UserConstructionScript`)