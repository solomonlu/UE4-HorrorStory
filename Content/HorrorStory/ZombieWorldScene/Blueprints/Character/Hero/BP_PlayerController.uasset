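; Player controller for both roles in a zombie game, Horror Master and hero, switched by IsHorrorMaster, which also adds the in-game HUD for the local player.
; The Horror Master spawns zombies under the cursor with right touch, limited by a cooldown counted down on Tick.
; Holding left touch opens a Tick-fed gate that drag-pans the commander pawn from its recorded start position.
; Otherwise, Tick rotates the hero toward the cursor's hit point.
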(event `self.ReceiveBeginPlay`
  (if (`self.IsLocalPlayerController` self)
    (bind _returnvalue (`|CreateWidget` "/Game/HorrorStory/ZombieWorldScene/Blueprints/UI/UI_HeroInGame.UI_HeroInGame_C" self))
    (`UserWidget.AddToViewport` _returnvalue 0)))

(event `SpawnZombie`
  (params (SpawnLocation :type "Vector Structure"))
  (`|SpawnActorFromClass` "/Game/HorrorStory/ZombieWorldScene/Blueprints/Character/Zombie/BP_Zombie.BP_Zombie_C" (`KismetMathLibrary.MakeTransform` SpawnLocation) "AdjustIfPossibleButAlwaysSpawn" "OverrideRootScale"))

(event `InputAction|RightTouch`
  (params (Key :type "Key Structure" :default "AnyKey"))
  (:`Pressed`
    (if (`self.IsHorrorMaster`)
      (if (<= (`self.CurrentSpawnCoolDown`) 0.0)
        (`self.SpawnZombie` (`.Location` (`GameplayStatics.BreakHitResult` (`self.GetHitResultUnderCursorByChannel` "TraceTypeQuery1"))))
        (set `self.CurrentSpawnCoolDown` (`self.SpawnCooldown`))))))

(event `InputAction|LeftTouch` :consume false
  (params (Key :type "Key Structure" :default "AnyKey"))
  (bind (_locationx _locationy) (`self.GetMousePosition`))
  (bind (_locationx_2 _locationy_2) (`self.GetMousePosition`))
  (bind (_returnvalue_x _returnvalue_y) (`KismetMathLibrary.BreakVector` (- (`self.TouchStartMousePosition`) (`KismetMathLibrary.MakeVector` _locationx_2 _locationy_2))))
  ;[1 1 1] Record mouse and commander position when touch start
  (:`Pressed`
    (set `self.TouchStartMousePosition` (`KismetMathLibrary.MakeVector` _locationx _locationy))
    (set `self.TouchStartCommanderPosition` (`self.K2_GetActorLocation` (`self.K2_GetPawn`)))
    (goto _label :!via `Open`))
  (:`Released`
    (goto _label :!via `Close`)))

(event `self.ReceiveTick`
  (params (DeltaSeconds :type "Float (single-precision)"))
  (bind (_locationx _locationy) (`self.GetMousePosition`))
  (bind (_returnvalue_x _returnvalue_y) (`KismetMathLibrary.BreakVector` (- (`self.TouchStartMousePosition`) (`KismetMathLibrary.MakeVector` _locationx _locationy))))
  (`|ExecutionSequence`
    (:`then_0`
      (`/Engine/EditorBlueprintResources/StandardMacros.IsValid` (`self.K2_GetPawn`)
        (:`Is Valid`
          (if (`self.IsHorrorMaster`)
            (`/Engine/EditorBlueprintResources/StandardMacros.Gate` true :!label _label ; While key is pressed...
              (:`Exit`
                (`self.K2_SetActorLocation` (`self.K2_GetPawn`) (+ (`self.TouchStartCommanderPosition`) (* (* (`KismetMathLibrary.MakeVector` _returnvalue_y (* _returnvalue_x -1.0 (`KismetMathLibrary.DegCos` 60.0))) -1.0) (`self.MouseMoveScale`))) false false)))
            (else
              ;[1 1 1] hero use mouse to rotate
              (`self.SetControlRotation` (`KismetMathLibrary.FindLookAtRotation` (`self.K2_GetActorLocation` (`self.K2_GetPawn`)) (`.Location` (`GameplayStatics.BreakHitResult` (`self.GetHitResultUnderCursorByChannel` "TraceTypeQuery1"))))))))))
    (:`then_1`
      (if (> (`self.CurrentSpawnCoolDown`) 0.0)
        (set `self.CurrentSpawnCoolDown` (- (`self.CurrentSpawnCoolDown`) DeltaSeconds))))))

(fn `UserConstructionScript`)