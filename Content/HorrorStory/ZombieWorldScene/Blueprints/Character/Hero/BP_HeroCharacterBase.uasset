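; Base hero character for a top-down, networked zombie shooter, with world-axis movement, weapon switching, a timed immortality shield and ragdoll death.
; The local player spawns fog of war and an aim target, projecting the cursor hit toward the camera to set aim height and control rotation.
; Server and multicast events drive firing, slot switching, shield and death.
; Bullets spawn on authority via WeaponComponent, and replicated health updates a bar.
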(event `self.ReceiveBeginPlay`
  (`|ExecutionSequence`
    (:`then_0`
      ;[1 1 1] add myself into ai storage
      (bind _outactors (`GameplayStatics.GetAllActorsOfClass` "/Game/AIBehaviorToolkit/Blueprints/BP_AIStorage.BP_AIStorage_C"))
      (if (> (`KismetArrayLibrary.Array_Length` _outactors) 0)
        (`/Game/AIBehaviorToolkit/Blueprints/BP_AIStorage.AddActorToList` (`KismetArrayLibrary.Array_Get` _outactors) self)))
    (:`then_1`
      (`KismetSystemLibrary.Delay` 0.5) ; wait a little time for possess compelete
      (if (`self.IsLocallyControlled`)
        ;[1 1 1] spawn fog of war
        (`|ExecutionSequence`
          (:`then_0`
            (bind _returnvalue (`|SpawnActorFromClass` "/Game/HorrorStory/Common/Blueprints/FogOfWar/BP_FogOfWar.BP_FogOfWar_C" (`KismetMathLibrary.MakeTransform` (0.0 0.0 0.0)) "Undefined" "OverrideRootScale"))
            (set `self.FogOfWar` _returnvalue))
          (:`then_1`
            ;[1 1 1] spawn gun aim target
            (bind _returnvalue_2 (`|SpawnActorFromClass` "/Game/HorrorStory/ZombieWorldScene/Blueprints/Character/Hero/BP_GunAimTarget.BP_GunAimTarget_C" (`KismetMathLibrary.MakeTransform` (0.0 0.0 0.0)) "Undefined" "OverrideRootScale"))
            (set `self.GunAimTarget` _returnvalue_2)))))))

(event `self.ReceiveTick`
  (params (DeltaSeconds :type "Float (single-precision)"))
  (bind _returnvalue (`PlayerCameraManager.GetCameraLocation` (`GameplayStatics.GetPlayerCameraManager` 0)))
  ;[1 1 1] set gun aim target
  (`self.GunAimTarget`
    (:`then`
      (bind _asplayer_controller (cast `PlayerController` (`self.GetController`)))
      (bind (_bblockinghit _binitialoverlap _time _location) (`GameplayStatics.BreakHitResult` (`PlayerController.GetHitResultUnderCursorByChannel` _asplayer_controller "TraceTypeQuery1" true)))
      (bind _returnvalue_2 (`KismetMathLibrary.VLerp` _location _returnvalue (/ (+ (`CapsuleComponent.GetScaledCapsuleHalfHeight` (`self.CapsuleComponent`)) (`self.BaseEyeHeight`)) (- (.z _returnvalue) (.z _location)))))
      (`self.K2_SetActorLocation` (`self.GunAimTarget`) _returnvalue_2 false false)
      (`Controller.SetControlRotation` _asplayer_controller (`KismetMathLibrary.FindLookAtRotation` (`self.GetActorEyesViewPoint`) _returnvalue_2)) ; set controller rotation
    )
    (:`else`)))

(event `OpenShield`
  ;[1 1 1] Shield
  (`self.MC_OpenShield`)
  (`Timeline|TimelineShield` :!via `PlayFromStart`
    (:`Finished`
      (`self.MC_CloseShield`))))

(event `self.ReceiveAnyDamage`
  (params (Damage :type "Float (single-precision)") (DamageType :type "DamageType Object Reference") (InstigatedBy :type "Controller Object Reference") (DamageCauser :type "Actor Object Reference"))
  ;[1 1 1] damage and death
  ;;[1 1 1] Reduce Health based on damage
  (if (not (`self.IsImmortal`))
    (bind _output_get (set `self.Health` (- (`self.Health`) Damage)))
    (if (<= _output_get 0.0)
      (`/Engine/EditorBlueprintResources/StandardMacros.DoOnce` false
        (:`Completed`
          (`self.MC_OnDeath`))))))

(event `MC_OpenShield`
  ;[1 1 1] Shield
  (set `self.IsImmortal` true)
  (`SceneComponent.SetHiddenInGame` (`self.ShieldMesh`) false false))

(event `MC_CloseShield`
  ;[1 1 1] Shield
  (set `self.IsImmortal` false)
  (`SceneComponent.SetHiddenInGame` (`self.ShieldMesh`) true false))

(event `MC_OnDeath`
  (bind _returnvalue (`self.GetController`))
  (bind _capsulecomponent (`self.CapsuleComponent`))
  (bind _mesh (`self.Mesh`))
  ;[1 1 1] damage and death
  (`|ExecutionSequence`
    (:`then_0`
      ;;[1 1 1] Default ragdoll death event
      (`PrimitiveComponent.SetCollisionResponseToAllChannels` _capsulecomponent "ECR_Ignore")
      (`PrimitiveComponent.SetCollisionResponseToChannel` _capsulecomponent "ECC_WorldStatic" "ECR_Block")
      (`PrimitiveComponent.SetCollisionProfileName` _mesh "Ragdoll")
      (`PrimitiveComponent.SetSimulatePhysics` _mesh true)
      (`AnimInstance.Montage_Stop` (`SkeletalMeshComponent.GetAnimInstance` _mesh) 0.0 null)
      ;;[1 1 1] clear tags
      (set `self.Tags` (`|MakeArray` "None" :!type "Name")))
    (:`then_1`
      ;;[1 1 1] disable owning client input and show game over widget
      (if (`KismetSystemLibrary.IsValid` _returnvalue)
        (if (`Controller.IsLocalPlayerController` _returnvalue)
          (`/Game/HorrorStory/ZombieWorldScene/Blueprints/GameModeEtc/BP_ZombieWorldPlayerController.NotifyHeroDown` (cast `/Game/HorrorStory/ZombieWorldScene/Blueprints/GameModeEtc/BP_ZombieWorldPlayerController` _returnvalue :!pure true)))))))

(event `SpawnBullet`
  (bind (_returnvalue_roll _returnvalue_pitch _returnvalue_yaw) (`KismetMathLibrary.BreakRotator` (`self.GetControlRotation`)))
  ;[1 1 1] bullet spawn, invoked by animation instance
  (`/Engine/EditorBlueprintResources/ActorMacros.Switch Has Authority`
    (:`Authority`
      (`/Game/HorrorStory/ZombieWorldScene/Blueprints/Character/Hero/Weapon/WeaponComponent.Server_SpawnBullet` (`self.WeaponComponent`) (`KismetMathLibrary.MakeRotator` 0.0 0.0 _returnvalue_yaw)))))

(event `self.ReceiveDestroyed`
  (`|ExecutionSequence`
    (:`then_0`
      (bind _fogofwar (`self.FogOfWar`)
        (:`then`
          (`self.K2_DestroyActor` _fogofwar))
        (:`else`)))
    (:`then_1`
      (bind _gunaimtarget (`self.GunAimTarget`)
        (:`then`
          (`self.K2_DestroyActor` _gunaimtarget))
        (:`else`)))))

(event `InputAxis|MoveForward`
  (params (AxisValue :type "Float (single-precision)"))
  ;[1 1 1] Movement
  (`self.AddMovementInput` (1.0 0.0 0.0) AxisValue))

(event `InputAxis|MoveRight`
  (params (AxisValue :type "Float (single-precision)"))
  ;[1 1 1] Movement
  (`self.AddMovementInput` (0.0 1.0 0.0) AxisValue))

(event `InputAction|Fire`
  (params (Key :type "Key Structure" :default "AnyKey"))
  ;[1 1 1] Fire
  (:`Pressed`
    (`self.Server_OnFire` true))
  (:`Released`
    (`self.Server_OnFire` false)))

(event `Server_OnFire`
  (params (IsAttacking :type Boolean))
  ;[1 1 1] Fire
  (`self.MC_OnFire` IsAttacking))

(event `MC_OnFire`
  (params (IsAttacking :type Boolean))
  ;[1 1 1] Fire
  (`/Game/HorrorStory/ZombieWorldScene/Blueprints/Character/Hero/Weapon/WeaponComponent.SetIsAttacking` (`self.WeaponComponent`) IsAttacking)
  (set `CharacterMovementComponent.bOrientRotationToMovement` (not IsAttacking) (`self.CharacterMovement`))
  (set `self.bUseControllerRotationYaw` IsAttacking))

(event `InputAction|EquipLastWeapon`
  (params (Key :type "Key Structure" :default "AnyKey"))
  ;[1 1 1] Equip weapon
  (:`Pressed`
    (`self.Server_EquipLastSlotWeapon`)))

(event `InputAction|EquipNextWeapon`
  (params (Key :type "Key Structure" :default "AnyKey"))
  ;[1 1 1] Equip weapon
  (:`Pressed`
    (`self.Server_EquipNextSlotWeapon`)))

(event `Server_EquipLastSlotWeapon`
  ;[1 1 1] Equip weapon
  (`/Game/HorrorStory/ZombieWorldScene/Blueprints/Character/Hero/Weapon/WeaponComponent.MC_SwitchWeaponSlot` (`self.WeaponComponent`) (cast `/Game/HorrorStory/ZombieWorldScene/Blueprints/Character/Hero/Weapon/Enum_WeaponSlotType` (- (`/Game/HorrorStory/ZombieWorldScene/Blueprints/Character/Hero/Weapon/WeaponComponent.GetCurrentActivingSlot` (`self.WeaponComponent`)) 1))))

(event `Server_EquipNextSlotWeapon`
  ;[1 1 1] Equip weapon
  (`/Game/HorrorStory/ZombieWorldScene/Blueprints/Character/Hero/Weapon/WeaponComponent.MC_SwitchWeaponSlot` (`self.WeaponComponent`) (cast `/Game/HorrorStory/ZombieWorldScene/Blueprints/Character/Hero/Weapon/Enum_WeaponSlotType` (+ (`/Game/HorrorStory/ZombieWorldScene/Blueprints/Character/Hero/Weapon/WeaponComponent.GetCurrentActivingSlot` (`self.WeaponComponent`)) 1))))

(fn `OnRep_Health`
  (`self.Update A Bar` "Health" (/ (`self.Health`) (`self.MaxHealth`))))

(fn `UserConstructionScript`)