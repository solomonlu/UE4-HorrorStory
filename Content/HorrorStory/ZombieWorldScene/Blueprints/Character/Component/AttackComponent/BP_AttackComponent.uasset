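; BP_AttackComponent handles weapon attacks for its owning Character in the zombie world.
; OnEquipWeapon loads the weapon's row from DT_WeaponParam by enum name and reports whether it was found.
; While IsAttacking, Tick plays that weapon's fire montage, using AttackSpeed as the countdown between plays.
; SpawnBullet spawns the weapon's projectile at a given transform, with no call to it in this graph.
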(event `self.ReceiveTick`
  (params (DeltaSeconds :type "Float (single-precision)"))
  (bind (_currentweaponparam_attackrangeddistance _currentweaponparam_attackspeed _currentweaponparam_numattacksbeforereload _currentweaponparam_fireanimations) (break `/Game/HorrorStory/ZombieWorldScene/Blueprints/Character/Hero/Weapon/Struct_WeaponParam` (`self.CurrentWeaponParam`)))
  (if (`self.IsAttacking`)
    ;[1 1 1] Play attack montage
    (bind _ascharacter (cast `Character` (`self.GetOwner`)))
    (if (<= (`self.CurrentAttackInterval`) 0.0)
      (`Character.PlayAnimMontage` _ascharacter _currentweaponparam_fireanimations 1.0 "None")
      (set `self.CurrentAttackInterval` _currentweaponparam_attackspeed)
      (else
        (set `self.CurrentAttackInterval` (- (`self.CurrentAttackInterval`) DeltaSeconds))))))

(fn `OnEquipWeapon`
  (params (NewWeapon :type "/Game/HorrorStory/ZombieWorldScene/Blueprints/Character/Hero/Weapon/Enum_WeaponType Enum"))
  (returns (Success :type Boolean))
  (bind _returnvalue (`|GetDataTableRow` "/Game/HorrorStory/ZombieWorldScene/Blueprints/Character/Hero/Weapon/DT_WeaponParam.DT_WeaponParam" (`KismetStringLibrary.Conv_StringToName` (`|GetEnumeratorNameAsString` NewWeapon)))
    (:`then`
      (set `self.CurrentWeaponParam` _returnvalue)
      (return true))
    (:`RowNotFound`
      (return false))))

(fn `SpawnBullet`
  (params (BulletTransform :type "Transform Structure"))
  (bind (_currentweaponparam_attackrangeddistance _currentweaponparam_attackspeed _currentweaponparam_numattacksbeforereload _currentweaponparam_fireanimations _currentweaponparam_reloadanimations _currentweaponparam_projectile) (break `/Game/HorrorStory/ZombieWorldScene/Blueprints/Character/Hero/Weapon/Struct_WeaponParam` (`self.CurrentWeaponParam`)))
  (`|SpawnActorFromClass` _currentweaponparam_projectile BulletTransform "Undefined" "OverrideRootScale"))