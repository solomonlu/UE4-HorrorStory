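; PickupEmitterComponent spawns a random pickup actor from a weighted list of pickup classes.
; RandomSpawnPickup sums the entry weights, rolls an integer from 1 to the total, then walks the list until the cumulative weight reaches the roll.
; It spawns that class at the given transform and returns the actor, or returns without spawning if the list is empty or the chosen class is invalid.
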(fn `RandomSpawnPickup`
  (params (InputPin :type "Transform Structure"))
  (returns (ReturnValue :type "/Game/HorrorStory/Common/Blueprints/Pickup/BP_PickupBase Object Reference"))
  (locals (TotalWeight :type Integer) (RandomWeight :type Integer) (CurrentWeight :type Integer))
  (if (> (`KismetArrayLibrary.Array_Length` (`self.PickupClass`)) 0)
    ;[1 1 1] calc total weight first
    (for _array_element (`self.PickupClass`)
      (set `local.TotalWeight` (+ (`.Weight_5_8FAB547D47CE23C8CA0FB691690C6D71` (break `/Game/HorrorStory/Common/Blueprints/Pickup/Struct_PickupEmitter` _array_element)) (`local.TotalWeight`))))
    ;[1 1 1] pick up a random weight
    (set `local.RandomWeight` (`KismetMathLibrary.RandomIntegerInRange` 1 (`local.TotalWeight`)))
    ;[1 1 1] if bigger than random weight , then pick it
    (for _array_element_2 (`self.PickupClass`)
      (bind (_pickupclass _weight) (break `/Game/HorrorStory/Common/Blueprints/Pickup/Struct_PickupEmitter` _array_element_2))
      (bind _output_get (set `local.CurrentWeight` (+ _weight (`local.CurrentWeight`))))
      (if (>= _output_get (`local.RandomWeight`))
        (if (`KismetSystemLibrary.IsValidClass` _pickupclass)
          (bind _returnvalue (`|SpawnActorFromClass` _pickupclass InputPin "Undefined" "OverrideRootScale"))
          (return _returnvalue)
          (else
            (return null)))))
    (else
      (return null))))