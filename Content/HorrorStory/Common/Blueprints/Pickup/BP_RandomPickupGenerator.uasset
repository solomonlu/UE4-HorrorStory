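; BP_RandomPickupGenerator is an actor that spawns a random pickup and replaces it after it is destroyed.
; On BeginPlay, with authority only, it asks its PickupEmitterComponent to spawn a pickup at the GeneratorPosition location with zero rotation.
; It binds to the spawned pickup's OnDestroyed event, which clears the reference, waits SpawnInterval and spawns again.
; The cycle continues only while each spawn returns a valid pickup, as a failed spawn schedules no retry.
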(event `self.ReceiveBeginPlay`
  (`self.SpawnPickup`))

(event `SpawnPickup`
  (`/Engine/EditorBlueprintResources/ActorMacros.Switch Has Authority`
    (:`Authority`
      (bind _returnvalue (`/Game/HorrorStory/Common/Blueprints/Pickup/PickupEmitterComponent.RandomSpawnPickup` (`self.PickupEmitterComponent`) (`KismetMathLibrary.MakeTransform` (`SceneComponent.K2_GetComponentLocation` (`self.GeneratorPosition`)))))
      (bind _output_get (set `self.SpawnedPickup` _returnvalue))
      (`/Engine/EditorBlueprintResources/StandardMacros.IsValid` _output_get
        (:`Is Valid`
          (add `self.OnDestroyed` _output_get (delegate `DelaySpawnPickup`)))))))

(event `DelaySpawnPickup` :!signature `self.OnDestroyed`
  (params (DestroyedActor :type "Actor Object Reference"))
  (set `self.SpawnedPickup` null)
  (`KismetSystemLibrary.Delay` (`self.SpawnInterval`))
  (`self.SpawnPickup`))

(fn `UserConstructionScript`)