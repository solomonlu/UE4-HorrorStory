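; BP_TeleportPoint is a teleport trigger that sends characters to a random actor of a configurable class.
; Calling Active unhides the PTeleportPoint component and arms the trigger.
; While armed, a Character overlapping the Sphere is teleported slightly above a randomly chosen TeleportToActorClass instance, using that actor's rotation.
; Destinations are gathered on each overlap, and nothing happens if the class is invalid or has no instances.
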(event `Active`
  (`SceneComponent.SetHiddenInGame` (`self.P_TeleportPoint`) false false)
  (set `self.IsActive` true))

(event `self.Sphere.OnComponentBeginOverlap`
  (params (OverlappedComponent :type "PrimitiveComponent Object Reference") (OtherActor :type "Actor Object Reference") (OtherComp :type "PrimitiveComponent Object Reference") (OtherBodyIndex :type Integer) (bFromSweep :type Boolean) (SweepResult :type "HitResult Structure (by ref)"))
  (if (`self.IsActive`)
    (cast `Character` OtherActor)
    (if (`KismetSystemLibrary.IsValidClass` (`self.TeleportToActorClass`))
      (bind _outactors (`GameplayStatics.GetAllActorsOfClass` (`self.TeleportToActorClass`)))
      (if (> (`KismetArrayLibrary.Array_Length` _outactors) 0)
        (bind (_returnvalue_location _returnvalue_rotation) (`KismetMathLibrary.BreakTransform` (`self.GetTransform` (`KismetArrayLibrary.Array_Get` _outactors (`KismetMathLibrary.RandomIntegerInRange` 0 (`KismetArrayLibrary.Array_LastIndex` _outactors))))))
        (`self.K2_TeleportTo` OtherActor (`KismetMathLibrary.MakeVector` (.x _returnvalue_location) (.y _returnvalue_location) (+ (.z _returnvalue_location) 50.0)) _returnvalue_rotation)))))

(fn `UserConstructionScript`)