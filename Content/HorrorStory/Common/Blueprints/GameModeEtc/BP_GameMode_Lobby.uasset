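; Lobby game mode that configures a multiplayer lobby from options passed by the main menu and enforces its player cap.
; BeginPlay parses the options string into the selected map and mode, max players, server name, and team-game and unique-selection flags.
; PostLogin and OnLogout track the player count, and a joiner over the limit is disconnected through the lobby player controller with a server-full reason.
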(event `self.ReceiveBeginPlay`
  ;[1 1 1] Parse all options that were passed from the MainMenu
  (`|ExecutionSequence`
    (:`then_0`
      (set `self.SelectedGamePlayMap` (`GameplayStatics.ParseOption` (`self.OptionsString`) "SelectedGamePlayMap")))
    (:`then_1`
      (set `self.SelectedGameMode` (`GameplayStatics.ParseOption` (`self.OptionsString`) "SelectedGameMode")))
    (:`then_2`
      (set `self.MaxNumPlayers` (`KismetStringLibrary.Conv_StringToInt` (`GameplayStatics.ParseOption` (`self.OptionsString`) "MaxNumPlayers"))))
    (:`then_3`
      (set `self.ServerName` (`GameplayStatics.ParseOption` (`self.OptionsString`) "ServerName")))
    (:`then_4`
      (switch `string` (`GameplayStatics.ParseOption` (`self.OptionsString`) "IsTeamGame")
        (:`true`
          (set `self.bIsTeamGame` true))
        (:`false`
          (set `self.bIsTeamGame` false))))
    (:`then_5`
      (switch `string` (`GameplayStatics.ParseOption` (`self.OptionsString`) "UniqueSelection")
        (:`true`
          (set `self.bOnlyUniqueSelection` true))
        (:`false`
          (set `self.bOnlyUniqueSelection` false))))))

(event `self.K2_PostLogin`
  (params (NewPlayer :type "PlayerController Object Reference"))
  ;[1 1 1] Higher and lower then Number when someone joins/leaves
  (bind _result (`/Engine/EditorBlueprintResources/StandardMacros.IncrementInt` (`self.CurrentNumberOfPlayers`))
    (:`  `
      ;[1 1 1] If we already reached the max number of players, send him back to the main-menu
      (if (and (> _result (`self.MaxNumPlayers`)) (> (`self.CurrentNumberOfPlayers`) 1))
        (bind _asbp_player_controller_lobby (cast `/Game/HorrorStory/Common/Blueprints/GameModeEtc/BP_PlayerController_Lobby` NewPlayer))
        (`/Game/HorrorStory/Common/Blueprints/GameModeEtc/BP_PlayerController_Lobby.ClientDisconnect` _asbp_player_controller_lobby true "Server is full!")))))

(event `self.K2_OnLogout`
  (params (ExitingController :type "Controller Object Reference"))
  ;[1 1 1] Higher and lower then Number when someone joins/leaves
  (`/Engine/EditorBlueprintResources/StandardMacros.DecrementInt` (`self.CurrentNumberOfPlayers`)))

(fn `UserConstructionScript`)