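; Rotating laser trap with two rods that each fire beams from two emitter sockets, damaging whatever they hit while active.
; BeginPlay spawns hidden beam particles at the sockets; Active and Deactive toggle their visibility and rotation.
; While active, Tick yaws the rods and line-traces from each socket, applying per-tick damage and setting beam endpoints.
; A test sequence in BeginPlay automatically switches the trap on after a delay, then off again.
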(event `/Game/HorrorStory/Common/Blueprints/TricksAndTraps/BPI_TricksAndTraps.Active`
  (set `self.IsActive` true)
  (for _array_element (`self.Lasers`)
    (`SceneComponent.SetHiddenInGame` _array_element false false)))

(event `self.ReceiveBeginPlay`
  (bind _rod2 (`self.Rod2`))
  (bind _rod1 (`self.Rod1`))
  (`|ExecutionSequence`
    (:`then_0`
      (`self.SpawnLaser` _rod1 "Emitter1"))
    (:`then_1`
      (`self.SpawnLaser` _rod1 "Emitter2"))
    (:`then_2`
      (`self.SpawnLaser` _rod2 "Emitter1"))
    (:`then_3`
      (`self.SpawnLaser` _rod2 "Emitter2"))
    (:`then_4`
      ;[1 1 1] Test
      (`KismetSystemLibrary.Delay` 2.0)
      (`self.Active`)
      (`KismetSystemLibrary.Delay` 10.0)
      (`self.Deactive`))))

(event `/Game/HorrorStory/Common/Blueprints/TricksAndTraps/BPI_TricksAndTraps.Deactive`
  (set `self.IsActive` false)
  (for _array_element (`self.Lasers`)
    (`SceneComponent.SetHiddenInGame` _array_element true false)))

(event `self.ReceiveTick`
  (params (DeltaSeconds :type "Float (single-precision)"))
  (bind _rod1 (`self.Rod1`))
  (bind _rod2 (`self.Rod2`))
  (bind _returnvalue (* DeltaSeconds (`self.RotateSpeed`)))
  (if (`self.IsActive`)
    (`|ExecutionSequence`
      (:`then_0`
        ;[1 1 1] rotate the rods
        (`SceneComponent.K2_AddRelativeRotation` (`self.Rod1`) (`KismetMathLibrary.MakeRotator` 0.0 0.0 _returnvalue) false false)
        (`SceneComponent.K2_AddRelativeRotation` (`self.Rod2`) (`KismetMathLibrary.MakeRotator` 0.0 0.0 _returnvalue) false false))
      (:`then_1`
        (`|ExecutionSequence`
          (:`then_0`
            (`self.TickLaser` _rod1 "Emitter1"))
          (:`then_1`
            (`self.TickLaser` _rod1 "Emitter2" 1))
          (:`then_2`
            (`self.TickLaser` _rod2 "Emitter1" 2))
          (:`then_3`
            (`self.TickLaser` _rod2 "Emitter2" 3)))))))

(fn `UserConstructionScript`)