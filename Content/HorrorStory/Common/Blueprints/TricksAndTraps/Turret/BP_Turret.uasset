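; BP_Turret is a timed trap turret that shoots projectiles at hero characters within its detection sphere and line of sight.
; Active plays a timeline that swings the Arrow from its pitched resting rotation, then reverses it through Deactive after ActiveTime.
; The timeline toggles three looping timers that pick a FocusTarget by overlap and Visibility trace, aim the Arrow at it and fire.
; Projectiles spawn only on the authority, ahead of the Arrow.
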(event `self.ReceiveBeginPlay`
  (`|ExecutionSequence`
    (:`then_0`
      (`SceneComponent.K2_SetWorldRotation` (`self.Arrow`) (`self.DefaultUnactiveRotation`) false false))
    (:`then_1`
      ;[1 1 1] Init Timer
      (bind _returnvalue (`KismetSystemLibrary.K2_SetTimer` null "TimerEvent_SpawnBullet" (`self.ShootingDelay`) true))
      (bind _output_get (set `self.ShootTimerHandler` _returnvalue))
      (`KismetSystemLibrary.K2_PauseTimerHandle` _output_get)
      (bind _returnvalue_2 (`KismetSystemLibrary.K2_SetTimer` null "TimerEvent_LookAtTarget" 0.01 true))
      (bind _output_get_2 (set `self.LookAtTargetTimerHandler` _returnvalue_2))
      (`KismetSystemLibrary.K2_PauseTimerHandle` _output_get_2)
      (bind _returnvalue_3 (`KismetSystemLibrary.K2_SetTimer` null "TimerEvent_CheckTargetLineInSight" 0.01 true))
      (bind _output_get_3 (set `self.Line Of Sight Timer` _returnvalue_3))
      (`KismetSystemLibrary.K2_PauseTimerHandle` _output_get_3))))

(event `TimerEvent_CheckTargetLineInSight`
  ;[1 1 1] Timer Event
  ;;[1 1 1] check current target line in sight
  (bind _focustarget (`self.FocusTarget`)
    (:`then`
      (bind _islineinsight (`self.CheckTargetLineInSight` _focustarget))
      (if (not (and (`PrimitiveComponent.IsOverlappingActor` (`self.CheckTargetSphere`) _focustarget) _islineinsight))
        (set `self.FocusTarget` null)
        ;;[1 1 1] pick up in CheckTargetSphere
        (for _array_element (`PrimitiveComponent.GetOverlappingActors` (`self.CheckTargetSphere`) "/Game/HorrorStory/ZombieWorldScene/Blueprints/Character/Hero/BP_HeroCharacterBase.BP_HeroCharacterBase_C") :!label _label
          (bind _islineinsight_2 (`self.CheckTargetLineInSight` _array_element))
          (if _islineinsight_2
            (set `self.FocusTarget` (cast `/Game/HorrorStory/ZombieWorldScene/Blueprints/Character/Hero/BP_HeroCharacterBase` _array_element :!pure true))
            (break)))))
    (:`else`
      (goto _label))))

(event `TimerEvent_LookAtTarget`
  ;[1 1 1] Timer Event
  (bind _focustarget (`self.FocusTarget`)
    (:`then`
      (`SceneComponent.K2_SetWorldRotation` (`self.Arrow`) (`KismetMathLibrary.FindLookAtRotation` (`self.K2_GetActorLocation`) (`self.K2_GetActorLocation` _focustarget)) false false))
    (:`else`)))

(event `/Game/HorrorStory/Common/Blueprints/TricksAndTraps/BPI_TricksAndTraps.Active`
  (set `self.IsActive` true)
  (`|ExecutionSequence`
    (:`then_0`
      (`KismetSystemLibrary.Delay` (`self.ActiveTime`))
      (`self.Deactive`))
    (:`then_1`
      ;[1 1 1] active the gun rotation
      (bind (_direction _lerp) (`Timeline|TimelineActive` :!label _label_2)
        (:`Update`
          (`SceneComponent.K2_SetWorldRotation` (`self.Arrow`) (`KismetMathLibrary.RLerp` (`self.DefaultUnactiveRotation`) (`self.DefaultActiveRotation`) _lerp true) false false))
        (:`Start`
          (`KismetSystemLibrary.K2_PauseTimerHandle` (`self.ShootTimerHandler`))
          (`KismetSystemLibrary.K2_PauseTimerHandle` (`self.LookAtTargetTimerHandler`))
          (`KismetSystemLibrary.K2_PauseTimerHandle` (`self.Line Of Sight Timer`)))
        (:`End`
          (`KismetSystemLibrary.K2_UnPauseTimerHandle` (`self.ShootTimerHandler`))
          (`KismetSystemLibrary.K2_UnPauseTimerHandle` (`self.LookAtTargetTimerHandler`))
          (`KismetSystemLibrary.K2_UnPauseTimerHandle` (`self.Line Of Sight Timer`)))))))

(event `/Game/HorrorStory/Common/Blueprints/TricksAndTraps/BPI_TricksAndTraps.Deactive`
  (set `self.IsActive` false)
  (goto _label_2 :!via `Reverse`))

(event `TimerEvent_SpawnBullet`
  (bind _arrow (`self.Arrow`))
  ;[1 1 1] Timer Event
  (`self.FocusTarget`
    (:`then`
      (`/Engine/EditorBlueprintResources/ActorMacros.Switch Has Authority`
        (:`Authority`
          (`|SpawnActorFromClass` "/Game/HorrorStory/Common/Blueprints/TricksAndTraps/Turret/BP_TurretProjectile.BP_TurretProjectile_C" (`KismetMathLibrary.MakeTransform` (+ (`SceneComponent.K2_GetComponentLocation` _arrow) (* (`SceneComponent.GetForwardVector` _arrow) (* (`ArrowComponent.ArrowSize` (`self.Arrow`)) 80.0))) (`SceneComponent.K2_GetComponentRotation` _arrow)) "Undefined" "OverrideRootScale"))))
    (:`else`)))

(fn `CheckTargetLineInSight`
  (params (Target :type "Actor Object Reference"))
  (returns (IsLineInSight :type Boolean))
  (bind _outhit (`KismetSystemLibrary.LineTraceSingle` (`self.K2_GetActorLocation`) (`self.K2_GetActorLocation` Target) "TraceTypeQuery1"))
  (bind (_bblockinghit _binitialoverlap _time _location _impactpoint _normal _impactnormal _physmat _hitactor) (`GameplayStatics.BreakHitResult` _outhit))
  (if _bblockinghit
    (return (== _hitactor Target))
    (else
      (return false))))

(fn `GetActive`
  (returns (IsActive :type Boolean))
  (return (`self.IsActive`)))

(fn `UserConstructionScript`
  (bind _output_get (set `self.DefaultActiveRotation` (`SceneComponent.K2_GetComponentRotation` (`self.Arrow`))))
  (set `self.DefaultUnactiveRotation` (`KismetMathLibrary.MakeRotator` (.roll _output_get) (- (.pitch _output_get) 30.0) (.yaw _output_get))))