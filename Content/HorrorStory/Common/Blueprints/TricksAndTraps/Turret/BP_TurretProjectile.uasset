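; BP_TurretProjectile is the projectile for the turret trap, dealing a fixed amount of damage on contact.
; Sphere overlaps damage a Character only when its capsule component is touched, then destroy the projectile; other overlaps are ignored.
; Blocking hits on the sphere damage any actor that can be damaged and always destroy the projectile.
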(event `self.Sphere.OnComponentBeginOverlap`
  (params (OverlappedComponent :type "PrimitiveComponent Object Reference") (OtherActor :type "Actor Object Reference") (OtherComp :type "PrimitiveComponent Object Reference") (OtherBodyIndex :type Integer) (bFromSweep :type Boolean) (SweepResult :type "HitResult Structure (by ref)"))
  (bind _ascharacter (cast `Character` OtherActor))
  (if (== OtherComp (`Character.CapsuleComponent` _ascharacter))
    (`GameplayStatics.ApplyDamage` _ascharacter 20.0)
    (`self.K2_DestroyActor`)))

(event `self.Sphere.OnComponentHit`
  (params (HitComponent :type "PrimitiveComponent Object Reference") (OtherActor :type "Actor Object Reference") (OtherComp :type "PrimitiveComponent Object Reference") (NormalImpulse :type "Vector Structure") (Hit :type "HitResult Structure (by ref)"))
  (if (`Actor.bCanBeDamaged` OtherActor)
    (`GameplayStatics.ApplyDamage` OtherActor 20.0))
  (`self.K2_DestroyActor`))

(fn `UserConstructionScript`)